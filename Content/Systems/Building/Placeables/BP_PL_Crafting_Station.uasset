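; Base-style crafting station placeable that forwards player interaction to its building scene components, with no ownership required.
; Outside dedicated servers, it listens for the crafting queue's artisan slot changes to show or hide a ThrallWorker mesh.
; An assigned thrall's character layout is applied through the customization component, refreshed when layout data arrives, and its animation plays.
; Getters expose artisan recipe and resource inventories; the artisan thrall inventory getter returns nothing.
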(event Custom|OnArtisanSlotChanged
  (params (thrallItem :type Thrall%20Item%20Object%20Reference))
  (Utilities|IsValid (Variables|Default|GetCurrentArtisanThrallItem)
    (:Is%20Valid
      (EventDispatchers|UnbindEventfromSignalReceivedCharacterLayout (stale _output_get) (delegate Custom|OnReceivedCharacterLayout)))
    (:Is%20Not%20Valid
      _))
  (bind _output_get (Variables|Default|SetCurrentArtisanThrallItem thrallItem))
  (Utilities|IsValid _output_get
    (:Is%20Valid
      (EventDispatchers|BindEventtoSignalReceivedCharacterLayout _output_get (delegate Custom|OnReceivedCharacterLayout))
      (Development|SetHiddeninGame (Variables|Default|GetThrallWorker) false true)
      (Class|CharacterCustomizationComponent|SetCharacterLayout (Variables|Default|GetBP_CharacterCustomizationComponent) (Variables|/Script/ConanSandbox.ThrallItem|GetThrallCharLayout (Variables|Default|GetCurrentArtisanThrallItem)) false false)
      (Components|Animation|PlayAnimation (Variables|Default|GetThrallWorker) (.animtoplay (Variables|/Script/Engine.SkeletalMeshComponent|GetAnimationData (Variables|Default|GetThrallWorker))) false))
    (:Is%20Not%20Valid
      (Development|SetHiddeninGame (Variables|Default|GetThrallWorker) true true))))

(event Custom|OnReceivedCharacterLayout
  (Development|SetHiddeninGame (Variables|Default|GetThrallWorker) false true)
  (Class|CharacterCustomizationComponent|SetCharacterLayout (Variables|Default|GetBP_CharacterCustomizationComponent) (Variables|/Script/ConanSandbox.ThrallItem|GetThrallCharLayout (Variables|Default|GetCurrentArtisanThrallItem)) false false)
  (Components|Animation|PlayAnimation (Variables|Default|GetThrallWorker) (.animtoplay (Variables|/Script/Engine.SkeletalMeshComponent|GetAnimationData (Variables|Default|GetThrallWorker))) false))

(event EventBeginPlay
  (|CallParentFunction)
  (if (not (Networking|IsDedicatedServer))
    (EventDispatchers|BindEventtoSignalArtisanSlotChanged (Variables|Default|GetCraftingQueue) (delegate Custom|OnArtisanSlotChanged))
    (Class|CharacterCustomizationComponent|SetMasterSkeletalMeshComponent (Variables|Default|GetBP_CharacterCustomizationComponent) (Variables|Default|GetThrallWorker) false)
    (Rendering|SetVisibility (Variables|Default|GetThrallWorker) false false)))

(event EventInteractableActivate
  (params (Component :type Primitive%20Component%20Object%20Reference) (Instigator :type Player%20Controller%20Object%20Reference) (HitIndex :type Integer))
  ;[1 1 1] WARLORDS: Interaction with crafting stations does not require ownership
  (for _array_element (Actor|GetComponentsByClass "/Game/Systems/Building/BuildingActorComponents/00_BP_SC_Building_MasterSceneComponent.00_BP_SC_Building_MasterSceneComponent_C")
    (Class|InteractableInterface|InteractableActivate _array_element Component Instigator HitIndex)))

(fn ConstructionScript
  (|CallParentFunction))

(fn GetArtisanRecipeInventory
  (return (Variables|Default|GetArtisanRecipeInventory)))

(fn GetArtisanThrallInventory
  (return 0))

(fn GetResourceInventory
  (return (Variables|Default|GetPlaceableInventory)))