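; Animation notify "AttackCollision" that signals the owning BaseBPCombat character that an attack's collision moment has been reached.
; Projectile weapons branch to ProjectileAttack, which now only checks locality and logs a missing player camera, without firing.
; The melee camera line trace, which would store hits on BP_CollisionComponent, is disconnected and never runs.
; Uncalled helpers play shield block sounds with a frontal-cone test and fetch a gathering component.
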(fn ReceivedNotify
  (params (MeshComp :type Skeletal%20Mesh%20Component%20Object%20Reference) (Animation :type Anim%20Sequence%20Base%20Object%20Reference))
  (bind _asbase_bpcombat (Utilities|Casting|CastToBaseBPCombat (Components|GetOwner MeshComp)))
  (bind _output_get (LocalVariables|SetAttackerCharacter _asbase_bpcombat))
  (Default|CallSignalAttackCollision _output_get)
  (bind _output_get_2 (LocalVariables|SetAttackWeapon (Default|GetWeaponItemActive _asbase_bpcombat)))
  (if (Utilities|DoesObjectImplementInterface _output_get_2 "/Game/Items/BP_ProjectileWeaponInterface.BP_ProjectileWeaponInterface_C")
    (CallFunction|ProjectileAttack (LocalVariables|GetAttackerCharacter))
    (return false)
    (elif (not (Networking|IsDedicatedServer))
      (return false)
      (else
        (return false)))))

(fn GetNotifyName
  (return "AttackCollision"))

(fn CheckDefenderAngle
  (params (Shield :type Base%20Weapon%20Object%20Reference) (Defender :type Base%20BP%20Combat%20Object%20Reference) (Attacker :type Base%20BP%20Combat%20Object%20Reference) (AttackerWeapon :type Base%20Weapon%20Object%20Reference))
  (Default|WeaponSoundImpactPlayBlock :self Shield :Attacker Attacker :Defender Defender :WhatHitMe AttackerWeapon)
  (return (<= (Class|KismetMathLibrary|DegAcos (Math|Vector|DotProduct (Transformation|GetActorForwardVector Defender) (Math|Vector|Normalize (- (Transformation|GetActorLocation Attacker) (Transformation|GetActorLocation Defender))))) 67.5)))

(fn GetGathering
  (params (Actor :type Actor%20Object%20Reference))
  (bind _returnvalue (Actor|GetComponentsByClass Actor "/Game/Systems/Survival/Gathering/BP_Gathering.BP_Gathering_C"))
  (if (> (Utilities|Array|Length _returnvalue) 0)
    (return (Utilities|Array|Get(acopy) _returnvalue))
    (else
      (return 0))))

(fn LineTraceHit
  (params (Attacker :type Base%20BP%20Combat%20Object%20Reference) (AttackerCollisionComponent :type BP%20Collision%20Component%20Object%20Reference))
  (bind _collisionmesh (Variables|Default|GetCollisionMesh))
  (bind _returnvalue (StaticMesh|GetBoundingBox _collisionmesh))
  (bind _max (Utilities|Struct|BreakBox _returnvalue))
  (bind _returnvalue_2 (Math|Vector|VectorLength _max))
  (LocalVariables|SetCollisionComponent AttackerCollisionComponent)
  (bind _isremote (Default|IsRemoteActor Attacker))
  (if _isremote
    (Variables|/Script/ConanSandbox.CollisionSystemComponent|SetHasDoneLineTrace (LocalVariables|GetCollisionComponent) true)
    (return)
    (else
      (LocalVariables|SetAttackingPlayer Attacker)
      (Utilities|IsValid (Default|GetWeaponItemPrimary (LocalVariables|GetAttackingPlayer))
        (:Is%20Valid
          (if (.Success (Default|GetVisualWeapon (Default|GetWeaponItemPrimary (LocalVariables|GetAttackingPlayer))))
            (Utilities|Array|Add (LocalVariables|GetActorsToIgnore) (.VisualActor (Default|GetVisualWeapon (Default|GetWeaponItemPrimary (LocalVariables|GetAttackingPlayer)))))))
        (:Is%20Not%20Valid
          _))
      (Utilities|IsValid (Default|GetWeaponItemSecondary (LocalVariables|GetAttackingPlayer))
        (:Is%20Valid
          (if (.Success (Default|GetVisualWeapon (Default|GetWeaponItemSecondary (LocalVariables|GetAttackingPlayer))))
            (Utilities|Array|Add (LocalVariables|GetActorsToIgnore) (.VisualActor (Default|GetVisualWeapon (Default|GetWeaponItemSecondary (LocalVariables|GetAttackingPlayer)))))))
        (:Is%20Not%20Valid
          _))
      (Utilities|Array|Add (LocalVariables|GetActorsToIgnore) (LocalVariables|GetAttackingPlayer))
      (bind (_outhit _returnvalue_3) (Collision|LineTraceByChannel (Transformation|GetWorldLocation (Utilities|Array|Get(acopy) (Actor|GetComponentsByClass (LocalVariables|GetAttackingPlayer) "/Script/ConanSandbox.AdjustableCameraComponent"))) (+ (Transformation|GetWorldLocation (Utilities|Array|Get(acopy) (Actor|GetComponentsByClass (LocalVariables|GetAttackingPlayer) "/Script/ConanSandbox.AdjustableCameraComponent"))) (* (Math|Vector|GetForwardVector (Utilities|Array|Get(acopy) (Actor|GetComponentsByClass (LocalVariables|GetAttackingPlayer) "/Script/ConanSandbox.AdjustableCameraComponent"))) (+ (* _returnvalue_2 2.0) (- (.Y (Math|Vector|BreakVector (.Location (Math|Transform|BreakTransform (Variables|Default|GetTransform))))) _returnvalue_2)))) "TraceTypeQuery1" true (LocalVariables|GetActorsToIgnore) "None"))
      (Utilities|IsValid (LocalVariables|GetCollisionComponent)
        (:Is%20Valid
          (if _returnvalue_3
            (Class|CollisionSystemComponent|AddLineTraceResult (LocalVariables|GetCollisionComponent) _outhit))
          (Variables|/Script/ConanSandbox.CollisionSystemComponent|SetLineTraceWasAHit (LocalVariables|GetCollisionComponent) _returnvalue_3))
        (:Is%20Not%20Valid
          _))
      (Variables|/Script/ConanSandbox.CollisionSystemComponent|SetHasDoneLineTrace (LocalVariables|GetCollisionComponent) true)
      (return))))

(fn ProjectileAttack
  (params (Attacker :type Base%20BP%20Combat%20Object%20Reference))
  (bind _inthirdperson (Variables|/Game/Characters/BaseBPCombat.BaseBPCombat_C|GetinThirdPerson Attacker))
  (bind _returnvalue (select _inthirdperson "ThirdPersonCamera" "FirstPersonCamera"))
  (if (not (Variables|/Game/Characters/BaseBPChar.BaseBPChar_C|GetIsNPC Attacker))
    (bind _isremote (Default|IsRemoteActor Attacker))
    (if (not _isremote)
      (if (not (> (Utilities|Array|Length (Actor|GetComponentsbyTag Attacker "/Script/Engine.CameraComponent" _returnvalue)) 0))
        (Class|LoggerLibrary|DWLogString (Utilities|String|Append "Failed to find camera with " (Utilities|String|ToString(Name) _returnvalue) " tag.") "Combat" "INFOL_DATAERROR")))
    (else
      ;[1 1 1] Kludge: IsRemoteActor prohibits NPCs from firing, so we use this instead.
      (if (Pawn|IsLocallyControlled Attacker)
        _))))