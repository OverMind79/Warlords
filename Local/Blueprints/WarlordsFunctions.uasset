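; Warlords function library with a function that calculates how much damage a weapon deals to a building piece.
; It reads the building's item tier from either an instanced building component or the actor's class, then compares it with the weapon item's tier.
; Only higher-tier melee weapons deal damage: two-handed maces and spears hit harder than one-handed types, and a one-tier advantage halves the result.
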(fn CalcBuildingDamage
  (params (Weapon :type Base%20Weapon%20Object%20Reference) (Component :type Primitive%20Component%20Object%20Reference) (Actor :type Actor%20Object%20Reference))
  (bind _owneritem (Variables|/Script/ConanSandbox.InventoryItemBase|GetOwnerItem Weapon))
  ;[0.1095 0.6413 1] Get Target Tier
  (bind _asinstanced_building_component (Utilities|Casting|CastToInstancedBuildingComponent Component)
    (:then
      (bind _returnvalue (Class|InstancedBuildingComponent|GetSourceClass _asinstanced_building_component))
      (bind _returnvalue_2 (Class|GameItemSpawner|FindBuildingItem _asinstanced_building_component _returnvalue))
      (LocalVariables|SettargetTier (.ItemTier (Utilities|Struct|BreakItemTableRow _returnvalue_2))))
    (:CastFailed
      (bind _returnvalue_3 (Class|GameItemSpawner|FindBuildingItem Actor (Utilities|GetClass Actor)))
      (LocalVariables|SettargetTier (.ItemTier (Utilities|Struct|BreakItemTableRow _returnvalue_3)))))
  (bind _output_get (LocalVariables|SetweaponTier (Class|GameItem|GetIntStat _owneritem "ItemTier")))
  (if (>= (- _output_get (LocalVariables|GettargetTier)) 1)
    (bind _asbpgame_item_weapon (Utilities|Casting|CastToBPGameItemWeapon _owneritem)
      (:then
        (if (or (Utilities|Enum|Equal(Enum) (Variables|/Game/Items/BPGameItemWeapon.BPGameItemWeapon_C|GetWeaponType _asbpgame_item_weapon) "Mace2H") (Utilities|Enum|Equal(Enum) (Variables|/Game/Items/BPGameItemWeapon.BPGameItemWeapon_C|GetWeaponType _asbpgame_item_weapon) "Spear2H"))
          (LocalVariables|SetdamageOutput 0.25)
          (if (>= (- _output_get (LocalVariables|GettargetTier)) 2) :!label _label
            (return (LocalVariables|GetdamageOutput))
            (else
              (return (* (LocalVariables|GetdamageOutput) 0.5))))
          (elif (Math|Boolean|ORBoolean (Utilities|Enum|Equal(Enum) (Variables|/Game/Items/BPGameItemWeapon.BPGameItemWeapon_C|GetWeaponType _asbpgame_item_weapon) "Sword") (Utilities|Enum|Equal(Enum) (Variables|/Game/Items/BPGameItemWeapon.BPGameItemWeapon_C|GetWeaponType _asbpgame_item_weapon) "Mace") (Utilities|Enum|Equal(Enum) (Variables|/Game/Items/BPGameItemWeapon.BPGameItemWeapon_C|GetWeaponType _asbpgame_item_weapon) "Spear") (Utilities|Enum|Equal(Enum) (Variables|/Game/Items/BPGameItemWeapon.BPGameItemWeapon_C|GetWeaponType _asbpgame_item_weapon) "Axe"))
            (LocalVariables|SetdamageOutput 0.1)
            (goto _label)
            (else
              _))))
      (:CastFailed
        _)))
  (return 0.0))