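; WeaponData provides functions that look up weapon stats and calculate health, stamina and concussive damage for players and NPCs.
; Player stats combine ItemTable and WlWeaponData rows, while NPC stats use ItemTable alone, both with fallback defaults.
; Player health damage scales with Might or Accuracy, while NPCs roll between tier and damage plus a bonus.
; One attack type raises the shared damage multiplier, blocking lowers it, and armor penetration is zero for NPCs.
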(fn WLGetPlayerWeaponData
  (params (TemplateID :type BP%20Game%20Item%20Object%20Reference))
  (bind _id (CallFunction|TemplateIDtoName (Variables|/Script/ConanSandbox.GameItem|GetTemplateID TemplateID)))
  (bind _returnvalue (Utilities|GetDataTableRow "/Game/Items/ItemTable.ItemTable" _id)
    (:then
      (bind _returnvalue_2 (Utilities|GetDataTableRow "/Game/Mods/Warlords/Tables/wlWeaponData.wlWeaponData" _id)
        (:then
          (return (.ItemTier (Utilities|Struct|BreakItemTableRow _returnvalue)) (.DamageMod (Utilities|Struct|BreakwlWeaponStruct _returnvalue_2)) (.DamageHealthLight_OnHit (Utilities|Struct|BreakItemTableRow _returnvalue)) (.DamageConcussiveLightOnHit (Utilities|Struct|BreakItemTableRow _returnvalue)) (.DamageStaminaLight_OnHit (Utilities|Struct|BreakItemTableRow _returnvalue)) (.ArmorPen (Utilities|Struct|BreakItemTableRow _returnvalue)) (.Speed (Utilities|Struct|BreakwlWeaponStruct _returnvalue_2)) (.ModType (Utilities|Struct|BreakwlWeaponStruct _returnvalue_2))))
        (:RowNotFound
          _)))
    (:RowNotFound
      _))
  (return 1 1.0 3 0 0 0.0 "NewEnumerator1" "NewEnumerator0"))

(fn WLCalculateWeaponDamage
  (params (Actor :type Actor%20Object%20Reference) (Attack%20Type :type SimpleAttack_AttackTypes%20Enum) (Weapon :type BP%20Game%20Item%20Weapon%20Object%20Reference) (Blocked :type Boolean) (Is%20NPC :type Boolean))
  (bind (_tier _bonus_damage _damage _con_damage _stamina_damage) (CallFunction|WLGetNPCWeaponData Weapon))
  (bind (_tier_2 _damage_mod _damage_2 _con_damage_2 _stamina_damage_2 _armor_pen _speed _modstat) (CallFunction|WLGetPlayerWeaponData Weapon))
  (Utilities|FlowControl|Sequence
    (:then_0
      (if Is%20NPC
        (LocalVariables|SetHDamage (Math|Conversions|ToFloat(Integer) (+ (Math|Random|RandomIntegerinRange _tier _damage) _bonus_damage)))
        (LocalVariables|SetCDamage (Math|Conversions|ToFloat(Integer) _con_damage))
        (LocalVariables|SetSDamage (Math|Conversions|ToFloat(Integer) _stamina_damage))
        (else
          (bind _asbase_player_char (Utilities|Casting|CastToBasePlayerChar Actor)
            (:then
              (if (Utilities|Enum|Equal(Enum) "NewEnumerator0" _modstat)
                (LocalVariables|SetHDamage (+ (Math|Conversions|ToFloat(Integer) _damage_2) (* (Variables|/Game/Systems/Progression/BP_ProgressionSystem.BP_ProgressionSystem_C|GetAttributeMight (Variables|/Game/Characters/BasePlayerChar.BasePlayerChar_C|GetBP_ProgressionSystem _asbase_player_char)) _damage_mod)))
                (else
                  (LocalVariables|SetHDamage (+ (Math|Conversions|ToFloat(Integer) _damage_2) (* (Variables|/Game/Systems/Progression/BP_ProgressionSystem.BP_ProgressionSystem_C|GetAttributeAccuracy (Variables|/Game/Characters/BasePlayerChar.BasePlayerChar_C|GetBP_ProgressionSystem _asbase_player_char)) _damage_mod)))))
              (LocalVariables|SetCDamage (Math|Conversions|ToFloat(Integer) _con_damage_2))
              (LocalVariables|SetSDamage (Math|Conversions|ToFloat(Integer) _stamina_damage_2)))
            (:CastFailed
              (return 0.0 0.0 0.0))))))
    (:then_1
      (if (Utilities|Enum|Equal(Enum) Attack%20Type "NewEnumerator1")
        (bind _output_get (LocalVariables|Setlocal%20Mod 1.5)))
      (if Blocked
        (LocalVariables|Setlocal%20Mod (- _output_get 0.75))))
    (:then_2
      (return (* (LocalVariables|Getlocal%20Mod) (LocalVariables|GetHDamage)) (* (LocalVariables|Getlocal%20Mod) (LocalVariables|GetSDamage)) (* (LocalVariables|Getlocal%20Mod) (LocalVariables|GetCDamage))))))

(fn GetNPCRow
  (params (InputPin :type Object%20Object%20Reference))
  (bind _outrownames (DataTable|GetDataTableRowNames "/Game/Mods/Warlords/Tables/wlWeaponData.wlWeaponData"))
  (bind _array_element (Utilities|Array|ForEachLoopwithBreak _outrownames :!label _label)
    (:LoopBody
      (bind _returnvalue (Utilities|GetDataTableRow "/Game/Mods/Warlords/Tables/wlWeaponData.wlWeaponData" _array_element)
        (:then
          (if (== (Utilities|GetClass InputPin) 0)
            (LocalVariables|SetResult _returnvalue)
            (LocalVariables|SetRow%20Found true)
            (goto _label Break)))))
    (:Completed
      (if (LocalVariables|GetRow%20Found)
        (return (LocalVariables|GetResult) (LocalVariables|GetRow%20Found))
        (else
          (return "" false))))))

(fn WLGetArmorPen
  (params (Actor :type Actor%20Object%20Reference) (Is%20NPC :type Boolean) (Weapon%20Template%20ID :type Integer))
  (if Is%20NPC
    (return 0.0)
    (else
      (return (.Armor%20Pen (CallFunction|WLGetPlayerWeaponData))))))

(fn WLGetNPCWeaponData
  (params (Weapon :type BP%20Game%20Item%20Object%20Reference))
  (bind _returnvalue (Utilities|GetDataTableRow "/Game/Items/ItemTable.ItemTable" (CallFunction|TemplateIDtoName (Variables|/Script/ConanSandbox.GameItem|GetTemplateID Weapon)))
    (:then
      (return (.ItemTier (Utilities|Struct|BreakItemTableRow _returnvalue)) (.DamageHealthHeavy_OnHit (Utilities|Struct|BreakItemTableRow _returnvalue)) (.DamageHealthLight_OnHit (Utilities|Struct|BreakItemTableRow _returnvalue)) (.DamageConcussiveLightOnHit (Utilities|Struct|BreakItemTableRow _returnvalue)) (.DamageStaminaLight_OnHit (Utilities|Struct|BreakItemTableRow _returnvalue)) (.ArmorPen (Utilities|Struct|BreakItemTableRow _returnvalue))))
    (:RowNotFound
      (return 1 0 3 0 0 0.0))))