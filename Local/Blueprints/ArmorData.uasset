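; ArmorData is a Blueprint set of lookup functions that read armor stats from the WlArmorData DataTable by row ID.
; Separate getters return an armor piece's Tier, Armor value and Weight, each through its own row lookup.
; Each getter also returns a Found flag, falling back to zero and false when the row is missing.
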(fn GetArmorTier
  (params (ID :type Name))
  (bind _returnvalue (Utilities|GetDataTableRow "/Game/Mods/Warlords/Tables/wlArmorData.wlArmorData" ID)
    (:then
      (return (Utilities|Struct|BreakwlArmorStruct _returnvalue) true))
    (:RowNotFound
      (return 0 false))))

(fn GetArmorArmor
  (params (ID :type Name))
  (bind _returnvalue (Utilities|GetDataTableRow "/Game/Mods/Warlords/Tables/wlArmorData.wlArmorData" ID)
    (:then
      (return (Utilities|Struct|BreakwlArmorStruct _returnvalue) true))
    (:RowNotFound
      (return 0.0 false))))

(fn GetArmorWeight
  (params (ID :type Name))
  (bind _returnvalue (Utilities|GetDataTableRow "/Game/Mods/Warlords/Tables/wlArmorData.wlArmorData" ID)
    (:then
      (return (Utilities|Struct|BreakwlArmorStruct _returnvalue) true))
    (:RowNotFound
      (return 0.0 false))))