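; Projectile weapon item that fires its active ammunition as a replicated projectile and accepts compatible ammo dropped onto it.
; Players draw ammo from shortcut bar, then backpack; NPCs, and players without ammo, get a spawned item instead.
; The wielder's aiming interface sets direction using projectile speed and a cheap min/max average of the gravity curve.
; The projectile receives that curve, community and computed damage, then weapon durability and any inventory ammo are reduced.
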(event EventProjectileAttack
  (params (CameraLocation :type Vector) (CameraRotation :type Rotator) (SocketLocation :type Vector) (SocketRotation :type Rotator))
  (CallFunction|ProjectileAttackImpl CameraLocation CameraRotation SocketLocation SocketRotation))

(fn ProjectileAttackImpl
  (params (CameraLocation :type Vector) (CameraRotation :type Rotator) (SocketLocation :type Vector) (SocketRotation :type Rotator))
  (bind (_visualactor _success) (CallFunction|GetVisualWeapon))
  (if _success
    (LocalVariables|Setlocal%20VisualWeapon _visualactor)
    (LocalVariables|Setlocal%20CombatBP (Default|GetCharacterOwner (LocalVariables|Getlocal%20VisualWeapon)))
    (LocalVariables|Setlocal%20CameraLocation CameraLocation)
    (LocalVariables|Setlocal%20CameraRotation CameraRotation)
    (LocalVariables|Setlocal%20SocketLocation SocketLocation)
    (LocalVariables|Setlocal%20SocketRotation SocketRotation)
    (LocalVariables|SetLocalActiveAmmoID (Class|GameItem|GetIntStat self "ActiveAmmunition"))
    (if (not (Variables|/Game/Characters/BaseBPChar.BaseBPChar_C|GetIsNPC (LocalVariables|Getlocal%20CombatBP)))
      ;[1 1 1] Get Ammo for Players
      (bind _returnvalue (Class|ConanCharacter|GetShortcutBarInventory (LocalVariables|Getlocal%20CombatBP)))
      (if (Class|ItemInventory|HasItembyTemplateID _returnvalue (LocalVariables|GetLocalActiveAmmoID) 1)
        (LocalVariables|Setlocal%20AmmoSourceInventory _returnvalue)
        (LocalVariables|Setlocal%20AmmoGameItem (Class|ItemInventory|GetItembyTemplateID (LocalVariables|Getlocal%20AmmoSourceInventory) (LocalVariables|GetLocalActiveAmmoID)) :!label _label)
        (else
          (bind _returnvalue_2 (Class|ConanCharacter|GetBackpackInventory (LocalVariables|Getlocal%20CombatBP)))
          (if (Class|ItemInventory|HasItembyTemplateID _returnvalue_2 (LocalVariables|GetLocalActiveAmmoID) 1)
            (LocalVariables|Setlocal%20AmmoSourceInventory _returnvalue_2)
            (goto _label)
            (else
              (bind _output_get (LocalVariables|SetLocalActiveAmmoID (Utilities|Array|Get(acopy) (Variables|Default|GetCompatableAmmunitions))))
              (bind _returnvalue_3 (Class|GameItemSpawner|SpawnGameItem _output_get))
              (LocalVariables|Setlocal%20AmmoGameItem _returnvalue_3)))))
      (else
        ;[1 1 1] Get Ammo for NPC's
        (bind _output_get_2 (LocalVariables|SetLocalActiveAmmoID (Math|Integer|SelectInt (LocalVariables|GetLocalActiveAmmoID) (Math|Integer|SelectInt (Utilities|Array|Get(acopy) (Variables|Default|GetCompatableAmmunitions)) (Class|KismetSystemLibrary|MakeLiteralInteger 53511) (Utilities|Array|IsValidIndex (Variables|Default|GetCompatableAmmunitions))) (> (LocalVariables|GetLocalActiveAmmoID) 0))))
        (bind _returnvalue_4 (Class|GameItemSpawner|SpawnGameItem _output_get_2))
        (LocalVariables|Setlocal%20AmmoGameItem _returnvalue_4)))
    (Utilities|IsValid (LocalVariables|Getlocal%20AmmoGameItem)
      (:Is%20Valid
        (bind _returnvalue_5 (Utilities|GetDataTableRow "/Game/Items/ItemTable.ItemTable" (Utilities|String|StringToName (Utilities|String|ToString(Integer) (LocalVariables|GetLocalActiveAmmoID))))
          (:then
            (LocalVariables|Setlocal%20AmmoVisualItem (Class|DreamworldBlueprints|GetClassDefaultObject (Utilities|ResolveSoftReference (.VisualObject (Utilities|Struct|BreakItemTableRow _returnvalue_5)))))
            ;[1 1 1] Get the initial proj speed and update it, this is needed to help NPC's aim
            (bind _asbpi_base_projectile (Utilities|Casting|CastToBPI_BaseProjectile (LocalVariables|Getlocal%20AmmoVisualItem))
              (:then
                (bind _value (Default|GetProjectileInitialSpeed _asbpi_base_projectile))
                (LocalVariables|Setlocal%20ProjectileInitialSpeed _value))
              (:CastFailed
                _))
            ;[1 1 1] Get average gravity value from curve;
            ; retrofitting this system to allow NPC's aim projectile weapons better;
            ; if the curve has extreme values NPC’s will have a hard time aiming the weapons, because we do not want to use differential math, expensive.
            (bind _projectileweapongravitycurve (Variables|Weapons|GetProjectileWeaponGravityCurve)
              (:then
                (LocalVariables|Setlocal%20ProjectileAverageGravity (|((Min+Max)*0.500000) (.MinValue (Class|CurveBase|GetValueRange _projectileweapongravitycurve)) (.MaxValue (Class|CurveBase|GetValueRange _projectileweapongravitycurve)))))
              (:else
                _))
            (bind _asbp_projectile_weapon_aiming_interface (Utilities|Casting|CastToBP_ProjectileWeaponAimingInterface (LocalVariables|Getlocal%20CombatBP)))
            (bind _launchdirection (Default|GetProjectileDirection _asbp_projectile_weapon_aiming_interface (LocalVariables|Getlocal%20CameraLocation) (LocalVariables|Getlocal%20CameraRotation) (LocalVariables|Getlocal%20SocketLocation) (LocalVariables|Getlocal%20SocketRotation) (Utilities|Array|MakeArray (LocalVariables|Getlocal%20CombatBP)) (LocalVariables|Getlocal%20ProjectileInitialSpeed) (LocalVariables|Getlocal%20ProjectileAverageGravity) 0.0))
            (LocalVariables|Setlocal%20ProjectileSpawn (|MakeProjectileSpawnTransform _launchdirection))
            (bind _returnvalue_6 (Class|GameItem|SpawnVisualItem (LocalVariables|Getlocal%20AmmoGameItem) (LocalVariables|Getlocal%20CombatBP) (LocalVariables|Getlocal%20ProjectileSpawn) "AlwaysSpawn" true))
            (Networking|SetReplicates _returnvalue_6 true)
            (bind _asbp_base_projectile (Utilities|Casting|CastToBP_BaseProjectile _returnvalue_6))
            (LocalVariables|Setlocal%20SpawnedVisualProjectile _asbp_base_projectile)
            (CallFunction|AffectDurabilityWeapon (LocalVariables|Getlocal%20VisualWeapon))
            (CallFunction|HandleProjectileGravityCurve (LocalVariables|Getlocal%20SpawnedVisualProjectile))
            ;[1 1 1] Calculate Damage + Community
            (Variables|/Game/Items/Weapons/BP_BaseProjectile.BP_BaseProjectile_C|SetCommunity (LocalVariables|Getlocal%20SpawnedVisualProjectile) (Variables|/Game/Characters/BaseBPChar.BaseBPChar_C|GetCommunity (LocalVariables|Getlocal%20CombatBP)))
            (Variables|/Game/Items/Weapons/BP_BaseProjectile.BP_BaseProjectile_C|SetDamage (LocalVariables|Getlocal%20SpawnedVisualProjectile) (CallFunction|WLCalculateProjectileWeaponDamage (LocalVariables|Getlocal%20AmmoGameItem) (Variables|/Script/ConanSandbox.InventoryItemBase|GetOwnerItem (LocalVariables|Getlocal%20VisualWeapon)) (LocalVariables|Getlocal%20CombatBP)))
            (Collision|IgnoreActorwhenMoving (Variables|/Game/Items/Weapons/BP_BaseProjectile.BP_BaseProjectile_C|GetCapsule (LocalVariables|Getlocal%20SpawnedVisualProjectile)) 0 false)
            ;[1 1 1] Remove ammo from the correct inventory, subtract from stack or remove single item stacks
            (Utilities|IsValid (LocalVariables|Getlocal%20AmmoSourceInventory)
              (:Is%20Valid
                (Class|ItemInventory|DeleteItemsbyTemplate (LocalVariables|Getlocal%20AmmoSourceInventory) (LocalVariables|GetLocalActiveAmmoID) 1))))))
      (:Is%20Not%20Valid
        (Utilities|DebugPrintSimple (Utilities|String|Append "XX_Projectile launch failed: Unable to create projectile " (Utilities|String|ToString(Integer) (LocalVariables|GetLocalActiveAmmoID))) "INFOL_CODEWARNING" "Combat")))))

(fn HasActiveAmmunition
  (bind _array_element (Utilities|Array|ForEachLoopwithBreak (Variables|Default|GetCompatableAmmunitions) :!label _label)
    (:LoopBody
      (if (== _array_element (Class|GameItem|GetIntStat "ActiveAmmunition"))
        (LocalVariables|Setlocal%20HasAmmoLoaded true)
        (goto _label Break)))
    (:Completed
      (return (LocalVariables|Getlocal%20HasAmmoLoaded)))))

(fn HandleProjectileLaunchLocation
  (bind _output_get (LocalVariables|Setlocal%20BaseWeapon (.VisualActor (CallFunction|GetVisualWeapon))))
  (bind _asbp_base_visual_projectile_weapon (Utilities|Casting|CastToBP_BaseVisualProjectileWeapon _output_get)
    (:then
      (return (Default|GetProjectileSocketLaunchLocation _asbp_base_visual_projectile_weapon)))
    (:CastFailed
      (Utilities|DebugPrintSimple (|MakeDebugString) "INFOL_CODEWARNING" "Combat"
        (:Output
          (return (Transformation|GetActorLocation (Default|GetCharacterOwner (LocalVariables|Getlocal%20BaseWeapon)))))))))

(fn OnItemDroppedonItem
  (params (droppedItem :type Game%20Item%20Object%20Reference) (srcInventory :type Item%20Inventory%20Object%20Reference) (srcIndex :type Integer))
  (bind _templateid (Variables|/Script/ConanSandbox.GameItem|GetTemplateID droppedItem))
  (if (Utilities|Enum|Equal(Enum) (Variables|/Script/ConanSandbox.GameItem|GetWeaponArcheType droppedItem) "Ammunition")
    (for _array_element (Variables|Default|GetCompatableAmmunitions)
      (if (== _array_element _templateid)
        (Class|GameItem|SetIntStat "ActiveAmmunition" _templateid true)
        (return true))))
  (return false))

(fn HandleProjectileGravityCurve
  (params (Projectile :type BP%20Base%20Projectile%20Object%20Reference))
  (bind _projectileweapongravitycurve (Variables|Weapons|GetProjectileWeaponGravityCurve)
    (:then
      (Variables|/Game/Items/Weapons/BP_BaseProjectile.BP_BaseProjectile_C|SetProjectileGravityCurve Projectile _projectileweapongravitycurve))
    (:else)))

(fn GetProjectileLaunchLocation
  (bind _output_get (LocalVariables|Setlocal%20BaseWeapon (.VisualActor (CallFunction|GetVisualWeapon))))
  (bind _asbp_base_visual_projectile_weapon (Utilities|Casting|CastToBP_BaseVisualProjectileWeapon _output_get)
    (:then
      (if (Utilities|IsValid (Variables|/Game/Items/Weapons/BaseWeapon.BaseWeapon_C|GetStaticWeaponMesh _asbp_base_visual_projectile_weapon))
        (return)
        (elif (Utilities|IsValid (Variables|/Game/Items/Weapons/BaseWeapon.BaseWeapon_C|GetWeaponSkeletalMesh _asbp_base_visual_projectile_weapon))
          (return)
          (else
            _))))
    (:CastFailed
      _))
  (Utilities|DebugPrintSimple (Utilities|String|ToString(Text) (Utilities|Text|FormatText "XX_Failed to get Socket_Projectile for {character} using {weapon}; reverting to the characters location to for spawning the projectile." (Utilities|Text|ToText(String) (Utilities|GetDisplayName (Default|GetCharacterOwner (LocalVariables|Getlocal%20BaseWeapon)))) (Utilities|Text|ToText(String) (Utilities|GetDisplayName (LocalVariables|Getlocal%20BaseWeapon))))) "INFOL_CODEWARNING" "Combat"
    (:Output
      (return))))